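; Bullet is a projectile actor that damages enemies it overlaps.
; Each Tick it moves along its forward vector at MoveSpeed without sweeping, and destroys itself once real time passes its Lifetime since BeginPlay.
; On overlap with an Enemy, it calls TakeDamage with a fixed amount and destroys itself, ignoring other actors.
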(event EventBeginPlay
  ;[1 1 1] Set Start Time
  (Variables|Default|SetStartTime (Utilities|Time|GetRealTimeSeconds)))

(event Collision|EventActorBeginOverlap
  (params (OtherActor :type Actor%20Object%20Reference))
  ;[1 1 1] Damage the Enemy
  (bind _asenemy (Utilities|Casting|CastToEnemy OtherActor))
  (Default|TakeDamage _asenemy 20)
  (Actor|DestroyActor))

(event EventTick
  (params (DeltaSeconds :type Float%20%28single-precision%29))
  ;[1 1 1] Moving Bullet & Destroying After Lifetime
  (Transformation|AddActorWorldOffset (* (Transformation|GetActorForwardVector) (* DeltaSeconds (Variables|Default|GetMoveSpeed))))
  (if (>= (Utilities|Time|GetRealTimeSeconds) (+ (Variables|Default|GetStartTime) (Variables|Default|GetLifetime)))
    (Actor|DestroyActor)))

(fn ConstructionScript)