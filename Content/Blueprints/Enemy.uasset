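; Enemy actor that chases the player, attacks at close range and can be killed.
; While alive, Tick turns its yaw toward the player and issues AIMoveTo, raising an Attacking flag for a fixed delay on arrival.
; AttackPlayer, not called in these graphs, damages the player if within range.
; TakeDamage reduces health and calls Die at zero, which sets Dead, disables capsule collision and halts movement.
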(event EventBeginPlay
  (bind _asplayer (Utilities|Casting|CastToPlayer (Game|GetPlayerCharacter 0)))
  (Variables|Default|SetPlayer _asplayer))

(event EventTick
  (params (DeltaSeconds :type Float%20%28single-precision%29))
  (if (not (Variables|Default|GetDead))
    (Utilities|FlowControl|Sequence
      (:then_0
        (Transformation|SetActorRotation (Math|Rotator|MakeRotator 0.0 0.0 (.Yaw (Math|Rotator|BreakRotator (Math|Rotator|FindLookatRotation (Transformation|GetActorLocation) (Transformation|GetActorLocation (Variables|Default|GetPlayer))))))))
      (:then_1
        (if (not (Variables|Default|GetAttacking))
          (AI|AIMoveTo self "0, 0, 0" (Variables|Default|GetPlayer) (Variables|Default|GetAttackStartDistance) false
            (:OnSuccess
              (if (not (Variables|Default|GetAttacking))
                (Variables|Default|SetAttacking true)
                (Utilities|FlowControl|Delay 2.6)
                (Variables|Default|SetAttacking false)))))))))

(fn ConstructionScript)

(fn AttackPlayer
  (if (<= (Math|Vector|Distance(Vector) (Transformation|GetActorLocation) (Transformation|GetActorLocation (Variables|Default|GetPlayer))) (Variables|Default|GetAttackMaxDistance))
    (Default|TakeDamage (Variables|Default|GetPlayer) (Variables|Default|GetDamage))))

(fn TakeDamage
  (params (DamageDealt :type Integer))
  (bind _output_get (Variables|Default|SetHealth (- (Variables|Default|GetHealth) DamageDealt)))
  (if (<= _output_get 0)
    (CallFunction|Die)))

(fn Die
  (Variables|Default|SetDead true)
  (Collision|SetCollisionEnabled (Variables|Collision|GetCapsuleComponent) "NoCollision")
  (Components|Movement|StopMovementImmediately (Variables|Character|GetCharacterMovement)))